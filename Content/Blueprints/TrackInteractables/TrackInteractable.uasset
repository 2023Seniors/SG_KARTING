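; Base-style track interactable actor that racers can activate while inside its trigger volume.
; Trigger overlap links it to the actor's PlayerTrackInteractability component as the current interactable and flags it in range, and end overlap clears both, with no racer check implemented.
; ExecuteInteraction sets IsActive and calls Interaction, a placeholder that prints debug text and resets IsActive, as any finished interaction must.
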(event `self.ReceiveTick`
  (params (DeltaSeconds :type "Float (single-precision)")))

(event `self.Trigger.OnComponentBeginOverlap`
  (params (OverlappedComponent :type "PrimitiveComponent Object Reference") (OtherActor :type "Actor Object Reference") (OtherComp :type "PrimitiveComponent Object Reference") (OtherBodyIndex :type Integer) (bFromSweep :type Boolean) (SweepResult :type "HitResult Structure (by ref)"))
  (bind _returnvalue (`self.GetComponentByClass` OtherActor "/Game/Blueprints/TrackInteractables/PlayerTrackInteractability.PlayerTrackInteractability_C"))
  (`KismetSystemLibrary.PrintText` "Event Linked To Player") ; Debug
  (set `/Game/Blueprints/TrackInteractables/PlayerTrackInteractability.IsInRangeOfInteraction` true _returnvalue)
  (set `/Game/Blueprints/TrackInteractables/PlayerTrackInteractability.CurrentInteractable` self _returnvalue))

(event `self.Trigger.OnComponentEndOverlap`
  (params (OverlappedComponent :type "PrimitiveComponent Object Reference") (OtherActor :type "Actor Object Reference") (OtherComp :type "PrimitiveComponent Object Reference") (OtherBodyIndex :type Integer))
  (bind _returnvalue (`self.GetComponentByClass` OtherActor "/Game/Blueprints/TrackInteractables/PlayerTrackInteractability.PlayerTrackInteractability_C"))
  (`KismetSystemLibrary.PrintText` "Event UNLIKED From Player")
  (set `/Game/Blueprints/TrackInteractables/PlayerTrackInteractability.IsInRangeOfInteraction` false _returnvalue) ; Set that racer is not in range of interaction anymore
  (set `/Game/Blueprints/TrackInteractables/PlayerTrackInteractability.CurrentInteractable` null _returnvalue) ; Set racer interactable to NULL (unlink)
)

(fn `ExecuteInteraction`
  (set `self.IsActive` true)
  (`self.Interaction`))

(fn `Interaction`
  (`KismetSystemLibrary.PrintString` "MICARA")
  ;[1 1 1] IMPORTANT: After an interactable action is finished, the interactable trigger has to be set back to innactive
  (set `self.IsActive` false))

(fn `UserConstructionScript`)