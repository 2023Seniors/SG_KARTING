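; PlayerTrackInteractability drives the player's use of track interactables, spending eligibility being gated by a MiguelitoBar value.
; Each Tick, while in interaction range, it calls ExecuteInteraction on CurrentInteractable if that is inactive and its Cost is strictly below MiguelitoBar.
; The input check is an always-true placeholder, so interactions fire automatically.
; This graph only reads the range flag, current interactable and bar, and never deducts the cost.
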(event `self.ReceiveTick`
  (params (DeltaSeconds :type "Float (single-precision)"))
  (bind _currentinteractable (`self.CurrentInteractable`))
  (if (`self.IsInRangeOfInteraction`)
    (if (< (`/Game/Blueprints/TrackInteractables/TrackInteractable.Cost` _currentinteractable) (`self.MiguelitoBar`))
      (if true
        (if (not (`/Game/Blueprints/TrackInteractables/TrackInteractable.IsActive` _currentinteractable))
          (`/Game/Blueprints/TrackInteractables/TrackInteractable.ExecuteInteraction` (`self.CurrentInteractable`)))))))