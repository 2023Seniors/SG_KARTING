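; ItemManager is an actor that tracks which track items are available and offers a random pick.
; On BeginPlay it registers with the L1_GameMode's GlobalReferenceBP, then rebuilds Items from the indices of true entries in AllItems.
; GetRandomItem returns a random position within Items, not the stored index, or -1 when empty.
; ResetAllItems writes each AllItems element back unchanged.
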(event `self.ReceiveBeginPlay`
  (`KismetSystemLibrary.PrintString` "WORKNIG")
  (`self.SubscribeManager`)
  (`self.UpdateItems`))

(fn `GetRandomItem`
  (returns (RandItem :type Integer))
  (bind _items (`self.Items`))
  (if (`KismetArrayLibrary.Array_IsEmpty` _items)
    (return -1)
    (else
      (return (`KismetMathLibrary.RandomInteger` (`KismetArrayLibrary.Array_Length` _items))))))

(fn `ResetAllItems`
  (bind _allitems (`self.AllItems`))
  (for (_array_element _array_index) _allitems
    (`KismetArrayLibrary.Array_Set` _allitems _array_index _array_element)))

(fn `SubscribeManager`
  (bind _asl1_game_mode (cast `/Game/Blueprints/L1_GameMode` (`GameplayStatics.GetGameMode`)))
  (`/Game/Blueprints/GlobalReferencesBP.SubscribeItemManager` (`/Game/Blueprints/L1_GameMode.Global Reference BP` _asl1_game_mode) self))

(fn `UpdateItems`
  (bind _items (`self.Items`))
  (`KismetArrayLibrary.Array_Clear` _items)
  (for (_array_element _array_index) (`self.AllItems`)
    (if _array_element
      (`KismetArrayLibrary.Array_Add` _items _array_index))))

(fn `UserConstructionScript`)