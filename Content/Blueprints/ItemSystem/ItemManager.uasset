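; ItemManager is an actor that tracks which items are active and supplies random picks.
; SetItem toggles a bounds-checked flag in the AllItems boolean array, and ResetAllItems turns every flag back on.
; UpdateItems rebuilds Items from the indices of active flags as a separate call.
; GetRandomItem returns a random position within Items, not the stored item index, or -1 when the list is empty.
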(fn `GetRandomItem`
  (returns (RandItem :type Integer))
  (bind _returnvalue (`KismetArrayLibrary.Array_Length` (`self.Items`)))
  (if (== _returnvalue 0)
    (return -1)
    (else
      (return (`KismetMathLibrary.RandomInteger` _returnvalue)))))

(fn `ResetAllItems`
  (bind _allitems (`self.AllItems`))
  (for (_ _array_index) _allitems
    (`KismetArrayLibrary.Array_Set` _allitems _array_index true)))

(fn `SetItem`
  (params (Item :type Integer) (Active :type Boolean))
  (bind _allitems (`self.AllItems`))
  (if (> (`KismetArrayLibrary.Array_Length` _allitems) Item)
    (`KismetArrayLibrary.Array_Set` _allitems Item Active)))

(fn `UpdateItems`
  (bind _items (`self.Items`))
  (`KismetArrayLibrary.Array_Clear` _items)
  (for (_array_element _array_index) (`self.AllItems`)
    (if _array_element
      (`KismetArrayLibrary.Array_Add` _items _array_index))))

(fn `UserConstructionScript`)