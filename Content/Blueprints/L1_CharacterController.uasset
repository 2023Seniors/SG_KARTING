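; Player controller for an arcade physics-driven vehicle (MiguelitoMobile) with drifting and boost.
; Enhanced Input drives forward force and steering; Tick applies smoothed, speed-scaled turning, drag, tilt clamping and speed-based camera distance.
; Drifting biases steering and alters drag, refilling boost faster; hit surface tags set damping.
; Also spawns spheres and line-traces to interact or push them; camera-look functions are unwired, and boost prints on screen.
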(event `self.ReceiveHit`
  (params (MyComp :type "PrimitiveComponent Object Reference") (Other :type "Actor Object Reference") (OtherComp :type "PrimitiveComponent Object Reference") (bSelfMoved :type Boolean) (HitLocation :type "Vector Structure") (HitNormal :type "Vector Structure") (NormalImpulse :type "Vector Structure") (Hit :type "HitResult Structure (by ref)"))
  (if (`ActorComponent.ComponentHasTag` OtherComp "On Road")
    (`PrimitiveComponent.SetLinearDamping` MyComp 1.0)
    (elif (`ActorComponent.ComponentHasTag` OtherComp "Off Road")
      (`PrimitiveComponent.SetLinearDamping` MyComp 2.5))))

(event `self.ReceiveBeginPlay`
  (`self.InitMappingContext`))

(event `self.ReceiveTick`
  (params (DeltaSeconds :type "Float (single-precision)"))
  (bind _booster_meter (`self.Booster_Meter`))
  (`self.Fix Rotation`)
  (`self.Angular Drag`)
  (`self.Update Rotation`)
  (`self.Add Turning`)
  (set `SpringArmComponent.TargetArmLength` (+ (* (`KismetMathLibrary.VSizeXY` (`SceneComponent.GetComponentVelocity` (`self.Miguelito_Mobile`))) 0.03) 300.0) (`self.SpringArm`))
  (if (!= (`self.DriftDir`) 0.0)
    (set `self.Booster_Meter` (`KismetMathLibrary.FMin` (+ (* (`GameplayStatics.GetWorldDeltaSeconds`) 10.0) (`self.Booster_Meter`)) 100.0))
    (else
      (set `self.Booster_Meter` (`KismetMathLibrary.FMin` (+ (* (`GameplayStatics.GetWorldDeltaSeconds`) 1.0) _booster_meter) 100.0))))
  (`KismetSystemLibrary.ExecuteConsoleCommand` "DisableAllScreenMessages " null)
  (`KismetSystemLibrary.ExecuteConsoleCommand` "EnableAllScreenMessages " null)
  (`KismetSystemLibrary.PrintString` (`KismetStringLibrary.BuildString_Int` "Boost Value: " "" (`KismetMathLibrary.FTrunc` _booster_meter)) true true (struct :`G` 0.66 :`B` 1.0 :`A` 1.0) 0.0))

(event `EnhancedInput|/Game/Inputs/Actions/L1_InputCamera`
  (params (ActionValue :type "Vector2D Structure") (ElapsedSeconds :type "Float (double-precision)") (TriggeredSeconds :type "Float (double-precision)") (InputAction :type "InputAction Object Reference" :default "/Game/Inputs/Actions/L1_InputCamera.L1_InputCamera")))

(event `EnhancedInput|/Game/Inputs/Actions/L1_InputMovement`
  (params (ActionValue :type "Vector2D Structure") (ElapsedSeconds :type "Float (double-precision)") (TriggeredSeconds :type "Float (double-precision)") (InputAction :type "InputAction Object Reference" :default "/Game/Inputs/Actions/L1_InputMovement.L1_InputMovement"))
  (bind _miguelito_mobile (`self.Miguelito_Mobile`))
  (:`Triggered`
    (if (not (== ActionValue_Y 0.0))
      (`PrimitiveComponent.AddForce` _miguelito_mobile (* (* (`SceneComponent.GetRightVector` _miguelito_mobile) (* (* (`self.MoveSpeed`) (* (- ActionValue_Y 0.1) 1.1)) 10000.0)) (1.0 1.0 0.0)) "None" false)
      (if (== (`self.DriftDir`) 0.0)
        (if (< ActionValue_Y 0.0)
          (set `self.Dir` (* ActionValue_X -1.0))
          (else
            (set `self.Dir` ActionValue_X)))
        (else
          (set `self.Dir` (+ (* (`self.DriftDir`) 0.65) (* ActionValue_X 0.35)))))))
  (:`Completed`
    (set `self.Dir` 0.0)))

(event `EnhancedInput|/Game/Inputs/Actions/L1_InputBoost`
  (params (ActionValue :type Boolean) (ElapsedSeconds :type "Float (double-precision)") (TriggeredSeconds :type "Float (double-precision)") (InputAction :type "InputAction Object Reference" :default "/Game/Inputs/Actions/L1_InputBoost.L1_InputBoost"))
  (bind _booster_meter (`self.Booster_Meter`))
  (bind _miguelito_mobile (`self.Miguelito_Mobile`))
  (:`Triggered`
    (if (> _booster_meter 1.0)
      (`PrimitiveComponent.AddForce` _miguelito_mobile (* (* (`SceneComponent.GetRightVector` _miguelito_mobile) (* (* (`self.MoveSpeed`) (* (- (`.Y` (`KismetMathLibrary.BreakVector2D` (stale `EnhancedInput|/Game/Inputs/Actions/L1_InputMovement` ActionValue))) 0.1) 1.1)) 10000.0)) (0.4 0.4 0.0)) "None" false)
      (set `self.Booster_Meter` (`KismetMathLibrary.FMax` (- _booster_meter (* (`GameplayStatics.GetWorldDeltaSeconds`) 40.0))))
      (`PrimitiveComponent.SetLinearDamping` (`self.Miguelito_Mobile`) 1.0))))

(event `EnhancedInput|/Game/Inputs/Actions/L1_InputSpawnBox`
  (params (ActionValue :type Boolean) (ElapsedSeconds :type "Float (double-precision)") (TriggeredSeconds :type "Float (double-precision)") (InputAction :type "InputAction Object Reference" :default "/Game/Inputs/Actions/L1_InputSpawnBox.L1_InputSpawnBox"))
  (bind _capsulecomponent (`self.CapsuleComponent`))
  (:`Started`
    (`|SpawnActorFromClass` "/Game/Spanwables/SpawnableSphereBP.SpawnableSphereBP_C" (`KismetMathLibrary.MakeTransform` (+ (* (`SceneComponent.GetForwardVector` _capsulecomponent) 1000.0) (`SceneComponent.K2_GetComponentLocation` _capsulecomponent))) "Undefined" "MultiplyWithRoot" null null)))

(event `EnhancedInput|/Game/Inputs/Actions/L1_InputAction`
  (params (ActionValue :type Boolean) (ElapsedSeconds :type "Float (double-precision)") (TriggeredSeconds :type "Float (double-precision)") (InputAction :type "InputAction Object Reference" :default "/Game/Inputs/Actions/L1_InputAction.L1_InputAction"))
  (bind _camera (`self.Camera`))
  (bind _returnvalue (`SceneComponent.K2_GetComponentLocation` _camera))
  (:`Started`
    (bind _outhit (`KismetSystemLibrary.LineTraceSingle` _returnvalue (+ _returnvalue (* (`SceneComponent.GetForwardVector` _camera) 100000.0)) "TraceTypeQuery1"))
    (bind (_bblockinghit _binitialoverlap _time _distance _location _impactpoint _normal _impactnormal _physmat _hitactor) (`GameplayStatics.BreakHitResult` _outhit))
    (`KismetSystemLibrary.PrintString` (`KismetStringLibrary.Concat_StrStr` "INTERACTED WITH : " (`KismetSystemLibrary.GetDisplayName` _hitactor)))
    (message `/Game/Interfaces/L1InteractInterface.DoSomethingAfterClicked` _hitactor)
    (bind _asspawnable_sphere_bp (cast `/Game/Spanwables/SpawnableSphereBP` _hitactor))
    (bind _retname (`/Game/Spanwables/SpawnableSphereBP.AddForcePromPlayer` _asspawnable_sphere_bp (`SceneComponent.GetForwardVector` (`self.CapsuleComponent`)) 500000.0))
    (`KismetSystemLibrary.PrintString` (`KismetStringLibrary.Concat_StrStr` _retname " has been pushed! "))))

(event `EnhancedInput|/Game/Inputs/Actions/L1_InputDrift`
  (params (ActionValue :type Boolean) (ElapsedSeconds :type "Float (double-precision)") (TriggeredSeconds :type "Float (double-precision)") (InputAction :type "InputAction Object Reference" :default "/Game/Inputs/Actions/L1_InputDrift.L1_InputDrift"))
  (bind _dir (`self.Dir`))
  (:`Started`
    (if (!= _dir 0.0)
      (set `self.DriftDir` _dir)
      (set `self.TurningVar` 0.0017)
      (set `self.DragVar` -500000.0)))
  (:`Completed`
    (set `self.TurningVar` 0.0012)
    (set `self.DragVar` -1000000.0)
    (set `self.DriftDir` 0.0)))

(fn `Add Turning`
  (bind _miguelito_mobile (`self.Miguelito_Mobile`))
  (bind _returnvalue (`KismetMathLibrary.FMin` (`KismetMathLibrary.VSizeXY` (`SceneComponent.GetComponentVelocity` _miguelito_mobile)) 2000.0))
  (if (< _returnvalue 1000.0)
    (`SceneComponent.K2_AddWorldRotation` _miguelito_mobile (`KismetMathLibrary.MakeRotator` 0.0 0.0 (* (`self.Rotation Speed`) (* (* _returnvalue 2.5) (`self.TurningVar`)))) false false)
    (else
      (`SceneComponent.K2_AddWorldRotation` _miguelito_mobile (`KismetMathLibrary.MakeRotator` 0.0 0.0 (* (`self.Rotation Speed`) (* (- 3000.0 (* _returnvalue 0.5)) (`self.TurningVar`)))) false false))))

(fn `Angular Drag`
  (bind _miguelito_mobile (`self.Miguelito_Mobile`))
  (bind _returnvalue (`KismetMathLibrary.Vector_Normal2D` (`SceneComponent.GetComponentVelocity` _miguelito_mobile)))
  (`PrimitiveComponent.AddForce` (`self.Miguelito_Mobile`) (* _returnvalue (* (`KismetMathLibrary.FMin` (- 1.0 (`KismetMathLibrary.Dot_VectorVector` _returnvalue (`KismetMathLibrary.Vector_Normal2D` (`SceneComponent.GetRightVector` _miguelito_mobile)))) 0.3) (`self.DragVar`))) "None" false))

(fn `Fix Rotation`
  (bind _miguelito_mobile (`self.Miguelito_Mobile`))
  (bind (_relativerotation_roll _relativerotation_pitch _relativerotation_yaw) (`KismetMathLibrary.BreakRotator` (`SceneComponent.RelativeRotation` _miguelito_mobile)))
  (`SceneComponent.K2_SetRelativeRotation` _miguelito_mobile (`KismetMathLibrary.MakeRotator` (`KismetMathLibrary.ClampAngle` _relativerotation_roll -30.0 30.0) (`KismetMathLibrary.ClampAngle` _relativerotation_pitch -30.0 30.0) _relativerotation_yaw) false false))

(fn `InitMappingContext`
  (`EnhancedInputSubsystemInterface.AddMappingContext` (pcsubsystem `EnhancedInputLocalPlayerSubsystem` (`GameplayStatics.GetPlayerController` 0)) "/Game/Inputs/L1_InputMapping.L1_InputMapping" 0 (struct)))

(fn `Update FPCamera`
  (params (A :type "Float (double-precision)") (B :type "Float (double-precision)"))
  (bind _camrotspeed (`self.CamRotSpeed`))
  (`SceneComponent.K2_AddLocalRotation` (`self.CapsuleComponent`) (`KismetMathLibrary.MakeRotator` 0.0 (* _camrotspeed B)) false false)
  (`self.AddControllerYawInput` (* A _camrotspeed)))

(fn `Update Rotation`
  (bind _springarm (`self.SpringArm`))
  (bind (_relativerotation_roll _relativerotation_pitch) (`KismetMathLibrary.BreakRotator` (`SceneComponent.RelativeRotation` _springarm)))
  (bind _output_get (set `self.Rotation Speed` (+ (* (`self.Dir`) 0.3) (* (`self.Rotation Speed`) 0.7))))
  (`SceneComponent.K2_SetRelativeRotation` _springarm (`KismetMathLibrary.MakeRotator` _relativerotation_roll _relativerotation_pitch (+ (* _output_get -5.0) 90.0)) false false))

(fn `Update3PCamera`
  (params (A :type "Float (double-precision)") (A2 :type "Float (double-precision)"))
  (bind _camrotspeed (`self.CamRotSpeed`))
  (`SceneComponent.K2_AddWorldRotation` (`self.SpringArm`) (`KismetMathLibrary.MakeRotator` 0.0 0.0 (* A _camrotspeed)) false false)
  (`SceneComponent.K2_AddLocalRotation` (`self.SpringArm`) (`KismetMathLibrary.MakeRotator` 0.0 (* A2 _camrotspeed)) false false))

(fn `UserConstructionScript`)